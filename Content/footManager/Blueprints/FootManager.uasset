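; FootManager is a Character component that produces footstep feedback and manages an optional circle decal under the character.
; FootManager traces downward, then optionally spawns a left/right decal aligned to ground normal and socket yaw, surface-specific sound, and Niagara or Cascade VFX.
; During falling, a looping timer projects the tagged circle decal onto the ground, optionally scaling it by height, until landing restores it.
; Event dispatchers expose each stage.
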(event EventBeginPlay
  ;[0 0 0] Event - Begin Play
  (bind _ascharacter (Utilities|Casting|CastToCharacter (Components|GetOwner))) ; Getting the parent of this actor component.
  (Variables|Default|SetCharacterReference _ascharacter) ; Create reference of the parent
  ;;[0 0 0] Circle Decal
  (CallFunction|InitializeCircleDecalValues) ; Initilialize Circle Decal Values when \nEnableCircleDecal is True
)

(fn FTraceLinetoFeet
  (params (DistanceToFeet :type Float%20%28double-precision%29))
  (bind _characterreference (Variables|Default|GetCharacterReference))
  (bind _returnvalue (Transformation|GetActorLocation _characterreference))
  (bind (_x _y _z) (Math|Vector|BreakVector _returnvalue))
  (bind (_outhit _returnvalue_2) (Collision|LineTraceByChannel _returnvalue (Math|Vector|MakeVector _x _y (- _z DistanceToFeet)) "TraceTypeQuery1" false 0 "None"))
  (if _returnvalue_2
    (Default|CallOnLineTracetoFeet _outhit))
  (return _outhit))

(fn FootManager
  (params (Foot%20Decal%20to%20Print :type E_Foot%20Enum :default "NewEnumerator0"))
  (if (Variables|Default|GetComponentActive?)
    (bind _outhit (FootManager|FTraceLinetoFeet (Utilities|Struct|BreakST_FootDecals (Variables|PrintFootStep|GetDecals%20Parameters))))
    (Variables|Private|SetOut%20Hit _outhit)
    (Utilities|FlowControl|Sequence
      (:then_0
        (if (Variables|PrintFootStep|GetPrintFootStepDecal)
          (FootManager|FPrintFootDecal Foot%20Decal%20to%20Print (Variables|Private|GetOut%20Hit))))
      (:then_1
        (if (Variables|PlayStepSound|GetPlayFootStepSound)
          (FootManager|FPlayFootStepSound (Variables|Private|GetOut%20Hit))))
      (:then_2
        (if (Variables|PlayStepVFX|GetPlayFootStepVFX)
          (FootManager|FPlayFootStepVFX (Variables|Private|GetOut%20Hit)))))))

(fn FPrintFootDecal
  (params (FootStep :type E_Foot%20Enum :default "NewEnumerator0") (OutHit :type Hit%20Result%20Structure))
  (bind (_bblockinghit _binitialoverlap _time _distance _location _impactpoint _normal) (Collision|BreakHitResult OutHit))
  (bind _decals_parameters (Variables|PrintFootStep|GetDecals%20Parameters))
  (bind _decals_parameters_2 (Variables|PrintFootStep|GetDecals%20Parameters))
  (bind _decals_parameters_3 (Variables|PrintFootStep|GetDecals%20Parameters))
  (bind (_leftfootdecalmaterial _rightfootdecalmaterial) (Utilities|Struct|BreakST_FootDecals _decals_parameters))
  (bind (_footdecalsize _footdecalduration) (Utilities|Struct|BreakST_FootDecals _decals_parameters_2))
  (bind (_leftfootsocketname _rightfootsocketname) (Utilities|Struct|BreakST_FootDecals _decals_parameters_3))
  (bind _returnvalue (Rendering|Decal|SpawnDecalatLocation (Utilities|Select :Index FootStep :NewEnumerator0 _leftfootdecalmaterial :NewEnumerator1 _rightfootdecalmaterial) _footdecalsize _impactpoint (Math|Rotator|MakeRotator 0.0 (.pitch (Math|Conversions|RotationFromXVector (Math|Vector|NegateVector _normal))) (+ (.yaw (Transformation|GetSocketRotation (Variables|/Script/Engine.Character|GetMesh (Variables|Default|GetCharacterReference)) (Utilities|Select :Index FootStep :NewEnumerator0 _leftfootsocketname :NewEnumerator1 _rightfootsocketname))) (Utilities|Struct|BreakST_FootDecals (Variables|PrintFootStep|GetDecals%20Parameters)))) _footdecalduration))
  (FootManager|FCallFootEvents _returnvalue FootStep))

(fn FCallFootEvents
  (params (DecalReference :type Decal%20Component%20Object%20Reference) (FootStep :type E_Foot%20Enum :default "NewEnumerator0"))
  (Default|CallOnFootPrinted DecalReference)
  (switch Utilities|FlowControl|Switch|SwitchonE_Foot FootStep
    (:NewEnumerator0
      (Default|CallOnLeftFootPrinted DecalReference))
    (:NewEnumerator1
      (Default|CallOnRightFootPrinted DecalReference))))

(fn FPlayFootStepVFX
  (params (OutHit :type Hit%20Result%20Structure))
  (bind _vfx_parameters (Variables|PlayStepVFX|GetVFX%20Parameters))
  (bind _vfx_parameters_2 (Variables|PlayStepVFX|GetVFX%20Parameters))
  (bind (_niagarasystem _particlesystem _rotation _scale) (Utilities|Struct|BreakST_FootVFX _vfx_parameters_2))
  (bind (_niagarasystem_2 _particlesystem_2 _rotation_2 _scale_2) (Utilities|Struct|BreakST_FootVFX _vfx_parameters))
  (switch Utilities|FlowControl|Switch|SwitchonE_FootVFX (Utilities|Struct|BreakST_FootVFX (Variables|PlayStepVFX|GetVFX%20Parameters))
    (:NewEnumerator0
      (Niagara|SpawnSystematLocation _niagarasystem (.ImpactPoint (Collision|BreakHitResult OutHit)) _rotation _scale))
    (:NewEnumerator1
      (Effects|SpawnEmitteratLocation _particlesystem_2 (.ImpactPoint (Collision|BreakHitResult OutHit)) _rotation_2 _scale_2)))
  (Default|CallOnVFXPlay (Utilities|Struct|BreakST_FootVFX (Variables|PlayStepVFX|GetVFX%20Parameters)) OutHit)
  (return))

(fn FPlayFootStepSound
  (params (OutHit :type Hit%20Result%20Structure))
  (bind _returnvalue (Collision|GetSurfaceType OutHit))
  (bind _sounds_parameters (Variables|PlayStepSound|GetSounds%20Parameters))
  (bind _sounds_parameters_2 (Variables|PlayStepSound|GetSounds%20Parameters))
  (bind (_rotation _volumemultiplier _pitchmultiplier _starttime _attenuationsettings _concurrencysettings _owningactor _initialparams) (Utilities|Struct|BreakST_FootStepSound _sounds_parameters))
  (bind _stepssoundslist (Utilities|Struct|BreakST_FootStepSound _sounds_parameters_2))
  (bind _value (Utilities|Map|Find _stepssoundslist _returnvalue))
  (Default|CallOnSoundPlay _value _returnvalue)
  (Audio|PlaySoundatLocation _value (.Location (Collision|BreakHitResult OutHit)) _rotation _volumemultiplier _pitchmultiplier _starttime _attenuationsettings _concurrencysettings _owningactor _initialparams)
  (return))

(fn FootManageronMovementModeChanged
  (params (Prev%20Movement%20Mode :type EMovementMode%20Enum :default "MOVE_None") (New%20Movement%20Mode :type EMovementMode%20Enum :default "MOVE_None"))
  (bind _decalinstance (Variables|Private|GetDecalInstance))
  (bind _circle_parameters (Variables|PrintCircleDecal|GetCircle%20Parameters))
  (bind _decalreference (Variables|Private|GetDecalReference))
  (bind _decalinstance_2 (Variables|Private|GetDecalInstance))
  (bind _circle_parameters_2 (Variables|PrintCircleDecal|GetCircle%20Parameters))
  (bind _sourcedecaltransform (Variables|Private|GetSourceDecalTransform))
  (bind _circleintensity (Utilities|Struct|BreakST_CircleDecal _circle_parameters))
  (bind _circlejumpintensity (Utilities|Struct|BreakST_CircleDecal _circle_parameters_2))
  (if (Variables|PrintCircleDecal|GetEnableCircleDecal)
    (Variables|Private|GetDecalReference
      (:then
        (if (and (Utilities|Enum|NotEqual(Enum) Prev%20Movement%20Mode "MOVE_Falling") (or (Utilities|Enum|Equal(Enum) New%20Movement%20Mode "MOVE_Falling") (Utilities|Enum|Equal(Enum) New%20Movement%20Mode "MOVE_None")))
          (bind _returnvalue (Utilities|Time|SetTimerbyFunctionName 0 "F_CircleDecalTick" (Utilities|Time|GetWorldDeltaSeconds) true))
          (Variables|Private|SetCircleDecalTickReference _returnvalue)
          (Rendering|Material|SetScalarParameterValue _decalinstance_2 "Intensity" _circlejumpintensity :!class /Script/Engine.MaterialInstanceDynamic)
          (Default|CallOnCircleJumpAnimationStarted _decalinstance_2 _circlejumpintensity (Variables|Private|GetCircleDecalTickReference))
          (elif (and (Utilities|Enum|Equal(Enum) Prev%20Movement%20Mode "MOVE_Falling") (Utilities|Enum|NotEqual(Enum) New%20Movement%20Mode "MOVE_Falling"))
            (Utilities|Time|ClearandInvalidateTimerbyHandle (Variables|Private|GetCircleDecalTickReference))
            (Transformation|SetRelativeLocation _decalreference (.location _sourcedecaltransform) false false)
            (Transformation|SetWorldScale3D _decalreference (.scale _sourcedecaltransform))
            (Rendering|Material|SetScalarParameterValue _decalinstance "Intensity" _circleintensity :!class /Script/Engine.MaterialInstanceDynamic)
            (Default|CallOnCircleJumpAnimationCompleted _decalinstance _circleintensity (Variables|Private|GetSourceDecalTransform)))))
      (:else))))

(fn InitializeCircleDecalValues
  (bind _characterreference (Variables|Default|GetCharacterReference))
  (bind _circle_parameters (Variables|PrintCircleDecal|GetCircle%20Parameters))
  (bind (_circledecaltag _circledecalmaterial _tracelinetofeetdistance _circleintensity _circlejumpintensity _circlecolor) (Utilities|Struct|BreakST_CircleDecal _circle_parameters))
  (bind _returnvalue (Actor|GetComponentsbyTag _characterreference "/Script/Engine.DecalComponent" _circledecaltag))
  (bind _output (Utilities|Array|Get(acopy) _returnvalue))
  (if (Variables|PrintCircleDecal|GetEnableCircleDecal)
    (Utilities|IsValid _output
      (:Is%20Valid
        (bind _output_get (Variables|Private|SetDecalReference _output))
        (Variables|Private|SetSourceDecalTransform (Transformation|GetRelativeTransform _output_get))
        (Rendering|Components|Decal|SetDecalMaterial _output_get _circledecalmaterial)
        (bind _returnvalue_2 (Rendering|Material|CreateDynamicMaterialInstance (Variables|Private|GetDecalReference) :!class /Script/Engine.DecalComponent))
        (bind _output_get_2 (Variables|Private|SetDecalInstance _returnvalue_2))
        (Rendering|Material|SetScalarParameterValue _output_get_2 "Intensity" _circleintensity :!class /Script/Engine.MaterialInstanceDynamic)
        (Rendering|Material|SetVectorParameterValue _output_get_2 "Color" _circlecolor :!class /Script/Engine.MaterialInstanceDynamic)
        (Default|CallOnCircleDecalInitialize (Variables|Private|GetDecalReference) (Variables|Private|GetDecalInstance) (Variables|Private|GetSourceDecalTransform) _circleintensity _circlecolor)))))

(fn FCircleDecalTick
  (bind _decalreference (Variables|Private|GetDecalReference))
  (bind _circle_parameters (Variables|PrintCircleDecal|GetCircle%20Parameters))
  (bind (_playcirclejumpanimation _jumpanimationscale) (Utilities|Struct|BreakST_CircleDecal _circle_parameters))
  (bind _outhit (FootManager|FTraceLinetoFeet (Utilities|Struct|BreakST_CircleDecal (Variables|PrintCircleDecal|GetCircle%20Parameters))))
  (Transformation|SetWorldLocation _decalreference (.ImpactPoint (Collision|BreakHitResult _outhit)) false false)
  (if _playcirclejumpanimation
    (Transformation|SetRelativeScale3D _decalreference (FootManager|FJumpAnimation (.ImpactPoint (Collision|BreakHitResult _outhit)) _jumpanimationscale)))
  (return))

(fn FJumpAnimation
  (params (Impact%20Point :type Vector) (JumpAnimationScale :type Float%20%28double-precision%29))
  (bind _characterreference (Variables|Default|GetCharacterReference))
  (bind _returnvalue (Transformation|GetActorLocation _characterreference))
  (bind _returnvalue_2 (- Impact%20Point _returnvalue))
  (bind _returnvalue_3 (Math|Vector|VectorLength _returnvalue_2))
  (bind _returnvalue_4 (Math|Float|NormalizetoRange _returnvalue_3 0.0 1e+02))
  (bind _returnvalue_5 (Math|Float|Clamp(Float) _returnvalue_4 0.0 JumpAnimationScale))
  (return (Math|Vector|MakeVector (.x (.scale (Variables|Private|GetSourceDecalTransform))) _returnvalue_5 _returnvalue_5)))